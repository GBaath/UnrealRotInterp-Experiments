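; BP_GB_OrbitCam is a mouse-driven orbit camera that delegates its movement to the BPACCameraMotionNew component.
; BeginPlay initializes the component on the Scene component's world location and sets Game and UI input mode.
; Temporary hardcoded mouse keys start and stop motion on press and release: left orbits, middle rotates statically, right dollies.
; Left and middle presses set the rotation mode first, while the right-button mode change is left unconnected.
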(event EventBeginPlay
  (Default|Init (Variables|Default|GetBPAC_CameraMotion_New) (Transformation|GetWorldLocation (Variables|Default|GetScene)) 0 "NewEnumerator1")
  (Input|SetInputModeGameandUI (Class|GameplayStatics|GetPlayerControllerfromID) 0 "DoNotLock" true false))

(event Input|MouseEvents|LeftMouseButton
  (params (Key :type Key%20Structure :default "None"))
  (bind _bpac_cameramotion_new (Variables|Default|GetBPAC_CameraMotion_New))
  ;[1 1 1] TEMP, replace with per-project input calls
  (:Pressed
    (Variables|/Game/ProductConfig/Blueprints/BPAC_CameraMotion_New.BPAC_CameraMotion_New_C|SetRotationMode _bpac_cameramotion_new "NewEnumerator1")
    (Default|StartOrbit _bpac_cameramotion_new))
  (:Released
    (Default|StopOrbit _bpac_cameramotion_new)))

(event Input|MouseEvents|MiddleMouseButton
  (params (Key :type Key%20Structure :default "None"))
  (bind _bpac_cameramotion_new (Variables|Default|GetBPAC_CameraMotion_New))
  ;[1 1 1] TEMP, replace with per-project input calls
  (:Pressed
    (Variables|/Game/ProductConfig/Blueprints/BPAC_CameraMotion_New.BPAC_CameraMotion_New_C|SetRotationMode _bpac_cameramotion_new "NewEnumerator0")
    (Default|StartStaticRotation _bpac_cameramotion_new))
  (:Released
    (Default|StopStaticRotation _bpac_cameramotion_new)))

(event Input|MouseEvents|RightMouseButton
  (params (Key :type Key%20Structure :default "None"))
  (bind _bpac_cameramotion_new (Variables|Default|GetBPAC_CameraMotion_New))
  ;[1 1 1] TEMP, replace with per-project input calls
  (:Pressed
    (Default|StartDolly _bpac_cameramotion_new))
  (:Released
    (Default|StopDolly _bpac_cameramotion_new)))

(fn ConstructionScript)