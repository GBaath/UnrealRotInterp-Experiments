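; Demo actor that compares rotation interpolation methods on a static mesh, driven through an on-screen stats widget.
; Start events pick a mode (constant or eased RInterp, rotator lerp, quaternion slerp, or eased slerp) and reset the mesh to its start rotation.
; Tick advances the active mode toward the target, blocks new starts until it finishes, and feeds the current rotator and quaternion to the widget.
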(event Custom|Slerp%20Quat%20Scaled
  ;[0 0.1583 0.7552] Quat Scaled
  (Variables|Default|SetAlpha (Math|Float|Clamp(Float) (Math|Interpolation|FInterpTo (Variables|Default|GetAlpha) 1.0 (Utilities|Time|GetWorldDeltaSeconds) (Variables|Default|GetSlerpSpeed))))
  (Transformation|SetWorldRotation (Variables|Default|GetStaticMesh) (Class|KismetMathLibrary|QuatRotator (Class|KismetMathLibrary|QuatSlerp (Variables|Default|GetStartQuat) (Variables|Default|GetTargetQuat) (Variables|Default|GetAlpha))) false false)
  (if (== (Variables|Default|GetAlpha) 1.0)
    (Variables|Default|SetRotationMode "NewEnumerator5")
    (Variables|Default|SetAlpha 0.0)))

(event Custom|Start%20interp%20rotator
  ;[1 0.7536 0.2678] Input
  (if (Variables|Default|GetCanClick)
    (Variables|Default|SetRotationMode "NewEnumerator2")
    (Transformation|SetWorldRotation (Variables|Default|GetStaticMesh) (Variables|Default|GetStartRot) false false)
    (Variables|Default|SetCanClick false)))

(event Custom|RInterp%20Rotator
  (bind _returnvalue (Utilities|Time|GetWorldDeltaSeconds))
  (bind _targetrot (Variables|Default|GetTargetRot))
  (bind _slerpspeed (Variables|Default|GetSlerpSpeed))
  (bind _staticmesh (Variables|Default|GetStaticMesh))
  (bind _returnvalue_2 (Transformation|GetWorldRotation _staticmesh))
  (bind _returnvalue_3 (Math|Interpolation|RInterpTo _returnvalue_2 _targetrot _returnvalue _slerpspeed))
  ;[0.1278 0.3073 0.1878] R interp
  (Transformation|SetWorldRotation (Variables|Default|GetStaticMesh) _returnvalue_3 false false)
  (if (Utilities|Operators|EqualEqual _returnvalue_3 (Variables|Default|GetTargetRot) 0.1)
    (Variables|Default|SetRotationMode "NewEnumerator5")))

(event Custom|SlerpQuat
  ;[0 0.08627 0.4115] Quat
  (Variables|Default|SetAlpha (Math|Float|Clamp(Float) (+ (Variables|Default|GetAlpha) (Utilities|Time|GetWorldDeltaSeconds))))
  (Transformation|SetWorldRotation (Variables|Default|GetStaticMesh) (Class|KismetMathLibrary|QuatRotator (Class|KismetMathLibrary|QuatSlerp (Variables|Default|GetStartQuat) (Variables|Default|GetTargetQuat) (Variables|Default|GetAlpha))) false false)
  (if (== (Variables|Default|GetAlpha) 1.0)
    (Variables|Default|SetAlpha 0.0)
    (Variables|Default|SetRotationMode "NewEnumerator5")))

(event Custom|StartQuatSlerp
  ;[1 0.7536 0.2678] Input
  (if (Variables|Default|GetCanClick)
    (Variables|Default|SetRotationMode "NewEnumerator0")
    (Transformation|SetWorldRotation (Variables|Default|GetStaticMesh) (Class|KismetMathLibrary|QuatRotator (Variables|Default|GetStartQuat)) false false)
    (Variables|Default|SetCanClick false)))

(event Custom|StartRotLerp
  ;[1 0.7536 0.2678] Input
  (if (Variables|Default|GetCanClick)
    (Variables|Default|SetRotationMode "NewEnumerator1")
    (Transformation|SetWorldRotation (Variables|Default|GetStaticMesh) (Variables|Default|GetStartRot) false false)
    (Variables|Default|SetCanClick false)))

(event Custom|interp%20const
  (bind _returnvalue (Utilities|Time|GetWorldDeltaSeconds))
  (bind _slerpspeed (Variables|Default|GetSlerpSpeed))
  (bind _targetrot (Variables|Default|GetTargetRot))
  (bind _staticmesh (Variables|Default|GetStaticMesh))
  (bind _returnvalue_2 (Transformation|GetWorldRotation _staticmesh))
  (bind _returnvalue_3 (* _slerpspeed 5.0))
  (bind _returnvalue_4 (Class|KismetMathLibrary|RInterptoConstant _returnvalue_2 _targetrot _returnvalue _returnvalue_3))
  ;[0 0.3073 0.1028] R interp const
  (Transformation|SetWorldRotation (Variables|Default|GetStaticMesh) _returnvalue_4 false false)
  (if (Utilities|Operators|EqualEqual _returnvalue_4 (Variables|Default|GetTargetRot) 0.1)
    (Variables|Default|SetRotationMode "NewEnumerator5")))

(event Custom|Start%20interp%20const
  ;[1 0.7536 0.2678] Input
  (if (Variables|Default|GetCanClick)
    (Variables|Default|SetRotationMode "NewEnumerator3")
    (Transformation|SetWorldRotation (Variables|Default|GetStaticMesh) (Variables|Default|GetStartRot) false false)
    (Variables|Default|SetCanClick false)))

(event Custom|LerpRotator
  ;[0.1758 0.2332 0.4688] Rotator
  (Variables|Default|SetAlpha (Math|Float|Clamp(Float) (+ (Variables|Default|GetAlpha) (Utilities|Time|GetWorldDeltaSeconds))))
  (Transformation|SetWorldRotation (Variables|Default|GetStaticMesh) (Math|Rotator|Lerp(Rotator) (Variables|Default|GetStartRot) (Variables|Default|GetTargetRot) (Variables|Default|GetAlpha)) false false)
  (if (== (Variables|Default|GetAlpha) 1.0)
    (Variables|Default|SetAlpha 0.0)
    (Variables|Default|SetRotationMode "NewEnumerator5")))

(event Custom|Start%20Quat%20Lerp%20Scaled
  ;[1 0.7536 0.2678] Input
  (if (Variables|Default|GetCanClick)
    (Variables|Default|SetRotationMode "NewEnumerator4")
    (Transformation|SetWorldRotation (Variables|Default|GetStaticMesh) (Class|KismetMathLibrary|QuatRotator (Variables|Default|GetStartQuat)) false false)
    (Variables|Default|SetCanClick false)))

(event EventTick
  (params (DeltaSeconds :type Float%20%28single-precision%29))
  (bind _staticmesh (Variables|Default|GetStaticMesh))
  (bind _returnvalue (Transformation|GetWorldRotation _staticmesh))
  ;[0.4635 0.2704 0.2882] Tick
  (Utilities|FlowControl|Sequence
    (:then_0
      (switch Utilities|FlowControl|Switch|SwitchonRotationMode (Variables|Default|GetRotationMode)
        (:NewEnumerator0
          (CallFunction|SlerpQuat))
        (:NewEnumerator1
          (CallFunction|LerpRotator))
        (:NewEnumerator2
          (CallFunction|RInterpRotator))
        (:NewEnumerator3
          (CallFunction|InterpConst))
        (:NewEnumerator4
          (CallFunction|SlerpQuatScaled))
        (:NewEnumerator5
          (Variables|Default|SetCanClick true))))
    (:then_1
      (Default|UpdateText (Variables|Default|GetUI) _returnvalue (Math|Conversions|ToQuaternion(Rotator) _returnvalue)))))

(event EventBeginPlay
  (bind _returnvalue (Class|GameplayStatics|GetPlayerControllerfromID))
  (bind _self self)
  (bind _returnvalue_2 (Transformation|GetActorRotation _self))
  ;[1 0.2135 0.2135] set start values
  (Variables|Default|SetStartRot _returnvalue_2)
  (Variables|Default|SetStartQuat (Math|Conversions|ToQuaternion(Rotator) _returnvalue_2))
  (bind _returnvalue_3 (UserInterface|CreateWidget "/Game/WBP_RotationStats.WBP_RotationStats_C" (Class|GameplayStatics|GetPlayerControllerfromID)))
  (bind _output_get (Variables|Default|SetUI _returnvalue_3))
  (Variables|/Game/WBP_RotationStats.WBP_RotationStats_C|SetRotatingA _output_get self)
  (UserInterface|Viewport|AddtoViewport _output_get 0)
  (Input|SetInputModeUIOnly _returnvalue (Variables|Default|GetUI) "DoNotLock" false)
  (Variables|/Script/Engine.PlayerController|SetbShowMouseCursor _returnvalue false))

(fn ConstructionScript)